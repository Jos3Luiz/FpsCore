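; First-person player character Blueprint that links the weapon inventory to the HUD and first-person animation.
; On BeginPlay it caches the first-person AnimBP and, for the locally controlled player, creates the HUD, which then follows ammo change events.
; Shoot animation transient events replay a timeline that drives additive recoil in the AnimBP.
; ReloadFix forwards to Reload, while the reload montage logic in the graph is disconnected.
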(event `ReloadFix`
  (`self.Reload`))

(event `self.WeaponInventory.OnAmmoChangeEvent`
  (params (CurrentAmmo :type Integer) (TotalAmmo :type Integer))
  (if (`self.IsLocallyControlled`)
    (`/Game/FpsCoreContent/UI/hud.UpdateAmmo` (`self.Hud`) CurrentAmmo TotalAmmo)))

(event `self.ReceiveBeginPlay`
  (`self.setup`)
  (`|ExecutionSequence`
    (:`then_1`
      (add `self.OnAnimTransientChangeEvent` (delegate `OnAnimTransientChangeEvent_Event_0`)))))

(event `OnAnimTransientChangeEvent_Event_0` :!signature `self.OnAnimTransientChangeEvent`
  (params (AnimationPoseIndex :type "EAnimEnumTransient Enum" :default "AET_Shoot"))
  (switch `EAnimEnumTransient` AnimationPoseIndex
    (:`AET_Shoot`
      ;[1 1 1] Recoil1
      (bind (_direction _recoil) (`Timeline|RecoilTL` :!via `PlayFromStart`)
        (:`Update`
          (set `/Game/FpsCoreContent/characters/FpsAnimBP/FirstPerson_AnimBP.aditionalRecoil1` (`KismetMathLibrary.MakeVector` (* _recoil -1.0)) (`self.FPSAnimBP`)))))))

(fn `setup`
  (set `self.FPSAnimBP` (cast `/Game/FpsCoreContent/characters/FpsAnimBP/FirstPerson_AnimBP` (`SkeletalMeshComponent.GetAnimInstance` (`self.FpsSkMesh`)) :!pure true))
  (if (`self.IsLocallyControlled`)
    (bind _returnvalue (`|CreateWidget` "/Game/FpsCoreContent/UI/hud.hud_C"))
    (bind _output_get (set `self.Hud` _returnvalue))
    (`UserWidget.AddToViewport` _output_get 0)
    (`/Game/FpsCoreContent/UI/hud.UpdateAmmo` (`self.Hud`) 0 0)))

(fn `UserConstructionScript`)